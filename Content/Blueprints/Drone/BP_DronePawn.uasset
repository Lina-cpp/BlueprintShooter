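; BP_DronePawn is a drone pawn that chases the player character and explodes on contact.
; A Sphere overlap with BP_FPSCharacter stores the target and starts AIMoveTo toward it.
; Tick smoothly rotates the drone to face the stored target using RInterpTo.
; An ExplodeSphere overlap with the player calls Explode, which plays sound and particle effects and destroys the drone, without applying damage.
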(event OnComponentBeginOverlap(Sphere)
  (params (OverlappedComponent :type Primitive%20Component%20Object%20Reference) (OtherActor :type Actor%20Object%20Reference) (OtherComp :type Primitive%20Component%20Object%20Reference) (OtherBodyIndex :type Integer) (bFromSweep :type Boolean) (SweepResult :type Hit%20Result%20Structure%20%28by%20ref%29))
  ;[1 1 1] Move to Player if in radius
  (bind _asbp_fpscharacter (Utilities|Casting|CastToBP_FPSCharacter OtherActor))
  (bind _output_get (Variables|Default|SetActor _asbp_fpscharacter))
  (AI|AIMoveTo self "0, 0, 0" _output_get 25.0 false))

(event OnComponentBeginOverlap(ExplodeSphere)
  (params (OverlappedComponent :type Primitive%20Component%20Object%20Reference) (OtherActor :type Actor%20Object%20Reference) (OtherComp :type Primitive%20Component%20Object%20Reference) (OtherBodyIndex :type Integer) (bFromSweep :type Boolean) (SweepResult :type Hit%20Result%20Structure%20%28by%20ref%29))
  ;[1 1 1] Explode on contact
  (Utilities|Casting|CastToBP_FPSCharacter OtherActor)
  (CallFunction|Explode))

(event EventBeginPlay)

(event Collision|EventActorBeginOverlap
  (params (OtherActor :type Actor%20Object%20Reference)))

(event EventTick
  (params (DeltaSeconds :type Float%20%28single-precision%29))
  (bind _actor (Variables|Default|GetActor))
  ;[1 1 1] Rotate Drone towards player
  (Utilities|IsValid _actor
    (:Is%20Valid
      (Transformation|SetActorRotation (Math|Interpolation|RInterpTo (Transformation|GetActorRotation) (Math|Rotator|FindLookatRotation (Transformation|GetActorLocation) (Transformation|GetActorLocation _actor)) DeltaSeconds 5.0)))))

(fn ConstructionScript)

(fn Explode
  (bind _returnvalue (Transformation|GetActorLocation))
  (Audio|PlaySoundatLocation "/Game/StarterContent/Audio/Explosion_Cue.Explosion_Cue" _returnvalue "0, 0, 0" 1.0 1.0 0.0 0 0 0 0)
  (Effects|SpawnEmitteratLocation "/Game/StarterContent/Particles/P_Explosion.P_Explosion" _returnvalue "0, 0, 0" "2.000000,2.000000,2.000000")
  (Actor|DestroyActor))